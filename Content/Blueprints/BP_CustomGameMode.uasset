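; Custom game mode Blueprint that manages the player-facing UI for a wave-based round game.
; It creates and shows the game interface widget at BeginPlay.
; The WaveOverBP event toggles the round timer and next-round button on that widget as waves end or begin.
; The GameOver event removes the interface and shows either the win or game-over screen.
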(event `self.ReceiveBeginPlay`
  (bind _returnvalue (`|CreateWidget` "/Game/Blueprints/UI/WBP_GameInterface.WBP_GameInterface_C"))
  (`UserWidget.AddToViewport` _returnvalue 0))

(event `self.ReceiveTick`
  (params (DeltaSeconds :type "Float (single-precision)")))

(event `self.WaveOverBP`
  (params (bIsOver :type Boolean))
  (if bIsOver
    (bind _roundtimer (`/Game/Blueprints/UI/WBP_GameInterface.RoundTimer` (stale `self.ReceiveBeginPlay` _returnvalue)))
    (`Widget.SetVisibility` _roundtimer "Visible")
    (`Widget.SetVisibility` (`/Game/Blueprints/UI/WBP_GameInterface.NextRoundButt` (stale `self.ReceiveBeginPlay` _returnvalue)) "Visible")
    (else
      (`Widget.SetVisibility` _roundtimer "Hidden")
      (`Widget.SetVisibility` (`/Game/Blueprints/UI/WBP_GameInterface.NextRoundButt` (stale `self.ReceiveBeginPlay` _returnvalue)) "Hidden"))))

(event `self.GameOver`
  (params (bWin :type Boolean))
  (`Widget.RemoveFromParent` (stale `self.ReceiveBeginPlay` _returnvalue))
  (if bWin
    (bind _returnvalue (`|CreateWidget` "/Game/Blueprints/UI/WBP_YouWin.WBP_YouWin_C"))
    (`UserWidget.AddToViewport` _returnvalue 0)
    (else
      (bind _returnvalue_2 (`|CreateWidget` "/Game/Blueprints/UI/WBP_GameOver.WBP_GameOver_C"))
      (`UserWidget.AddToViewport` _returnvalue_2 0))))

(fn `UserConstructionScript`)