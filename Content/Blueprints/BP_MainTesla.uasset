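; BP_MainTesla is a Tesla coil Blueprint that supplies the visual and audio effects for its lightning attack.
; CreateLightningFX spawns an auto-destroying Niagara beam attached to the capsule, running from the firing point to the target.
; The beam end is pushed out along the impact normal, which is also passed to the system, and a zap sound plays.
; Targeting and damage are not handled in this graph.
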(event `self.ReceiveTick`
  (params (DeltaSeconds :type "Float (single-precision)")))

(event `self.CreateLightningFX`
  (params (startPoint :type "Vector Structure") (targetPosition :type "Vector Structure") (impactNormal :type "Vector Structure"))
  ;[1 1 1] Spawn System and Set Niagara Variables
  (bind _returnvalue (`NiagaraFunctionLibrary.SpawnSystemAttached` "/Game/Assets/CoilEffect/NS_LightningAtack.NS_LightningAtack" (`self.CapsuleComp`) "None" (0.0 0.0 0.0) (struct) "KeepRelativeOffset" true))
  (`NiagaraComponent.SetVariableVec3` _returnvalue "BeamStartPoint" (`SceneComponent.K2_GetComponentLocation` (`self.FiringPoint`)))
  (`NiagaraComponent.SetVariableVec3` _returnvalue "BeamEndPoint" (+ targetPosition (* impactNormal (`self.ImpactOffset`))))
  (`NiagaraComponent.SetVariableVec3` _returnvalue "ImpactNormal" impactNormal)
  (`GameplayStatics.PlaySoundAtLocation` "/Game/Assets/CoilEffect/Sound/CoilZap_FX.CoilZap_FX" (0.0 0.0 0.0) (struct) 0.4 1.0 0.0 null null null null))

(fn `UserConstructionScript`)